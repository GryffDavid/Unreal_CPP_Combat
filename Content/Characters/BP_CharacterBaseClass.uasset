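; Base player character class for KOTOR-style combat with active pause and a dialogue camera.
; On its turn, Tick runs queued actions after a short delay, then ends the encounter turn; an emptied queue refills with a ranged attack mirrored in the UI.
; Attacks roll d20 against defense, then fire bolts carrying hit and damage results, with aim offsets faking misses.
; Incoming bolts flagged to hit trigger reactions and sparks, without applying damage.
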(event Custom|ToggleActivePause
  (Game|SetGamePaused (not (Game|IsGamePaused)))
  (Variables|/Script/Engine.CameraComponent|SetPostProcessSettings (Variables|Default|GetCamera) (Utilities|Struct|MakePostProcessSettings 1.0 0.0 15.0 15.0 0.0)))

(event EventTick
  (params (DeltaSeconds :type Float%20%28single-precision%29))
  (bind _actionarray (Variables|Default|GetActionArray))
  (if (Variables|Default|GetInCombat)
    (if (Variables|Default|GetIsMyTurn)
      (bind _output_get (Variables|Default|SetTimeSinceLastAction (+ DeltaSeconds (Variables|Default|GetTimeSinceLastAction))))
      (if (and (>= _output_get 0.8) (> (Utilities|Array|Length _actionarray) 0))
        (switch Utilities|FlowControl|Switch|SwitchonActionTypes (Utilities|Array|Get(acopy) _actionarray)
          (:NewEnumerator0
            (CallFunction|RangedAttackFunction)
            (CallFunction|RemoveFinishedAction)
            (Variables|Default|SetTimeSinceLastAction 0.0)
            (Variables|Default|SetIsMyTurn false)
            (Default|EndTurnEvent (Variables|Default|GetCurrentCombatEncounter))))))))

(event Collision|EventActorBeginOverlap
  (params (OtherActor :type Actor%20Object%20Reference))
  ;[1 1 1] Overlapped with Blaster bolt. Ignore if is not current target or shot is meant to miss
  (bind _asbp_enemy_blaster_bolt_projectile (Utilities|Casting|CastToBP_EnemyBlasterBoltProjectile OtherActor))
  (if (Variables|/Script/Unreal_CPP_Combat.BlasterBoltProjectile|GetCanHit _asbp_enemy_blaster_bolt_projectile)
    (if false
      _
      (else
        _))
    (CallFunction|HitbyBlaster)
    (Effects|SpawnEmitteratLocation "/Game/P_Sparks.P_Sparks" (Transformation|GetActorLocation _asbp_enemy_blaster_bolt_projectile))
    (Actor|DestroyActor _asbp_enemy_blaster_bolt_projectile)))

(event EventBeginPlay
  (bind _returnvalue (Game|GetPlayerController 0))
  (Input|SetInputModeGameandUI _returnvalue 0 "LockOnCapture" true)
  (Variables|/Script/Engine.PlayerController|SetbShowMouseCursor _returnvalue true))

(event Input|ActionEvents|InputActionJump
  (params (Key :type Key%20Structure))
  ;[1 1 1] Pause Game Mode. For KOTOR-style active pause.
  (:Pressed
    (CallFunction|ToggleActivePause)))

(fn ConstructionScript
  (Components|Activation|SetAutoActivate (Variables|Default|GetCamera) true)
  (Components|Activation|SetAutoActivate (Variables|Default|GetDialogueCamera) false))

(fn RangedAttackFunction
  (bind _targetedenemy (Variables|Default|GetTargetedEnemy))
  (bind _gunbarrel (Variables|Default|GetGunBarrel))
  (bind _returnvalue (Transformation|GetWorldLocation _gunbarrel))
  (bind _asbp_enemy_base_class (Utilities|Casting|CastToBP_EnemyBaseClass _targetedenemy))
  (bind _returnvalue_2 (Class|DiceRoll|RollD20vDC (Variables|/Script/Unreal_CPP_Combat.EnemyBaseClass|GetDefense _asbp_enemy_base_class) 0 1))
  (bind _returnvalue_3 (CallFunction|AddRandomMiss _returnvalue_2))
  (if _returnvalue_2
    (bind _returnvalue_4 (Class|DiceRoll|RollD6 1)))
  (Game|SpawnActorfromClass "/Game/Blueprints/BP_BlasterBoltProjectile.BP_BlasterBoltProjectile_C" (Math|Transform|MakeTransform _returnvalue (Math|Conversions|RotationFromXVector (Math|Vector|GetUnitDirection(Vector) _returnvalue (+ (Transformation|GetWorldLocation (Variables|/Game/Enemies/BP_EnemyBaseClass.BP_EnemyBaseClass_C|GetChestMarker _asbp_enemy_base_class)) _returnvalue_3)))) "Undefined" 0 _returnvalue_2 _returnvalue_4 0)
  (switch Utilities|FlowControl|Switch|SwitchonWeaponTypes (Variables|Default|GetEquippedWeaponType)
    (:NewEnumerator0
      (Animation|PlayAnimMontage "/Game/AnimStarterPack/ShootPistol.ShootPistol" 1.0 "None"))
    (:NewEnumerator1
      (Animation|PlayAnimMontage "/Game/AnimStarterPack/Shoot.Shoot" 1.8 "None"))))

(fn AddRandomMiss
  (params (Hit :type Boolean))
  (bind _returnvalue (Math|Random|RandomFloatinRange -1.1e+02 1.1e+02))
  (bind _returnvalue_2 (Math|Random|RandomFloatinRange 0.0 3.6e+02))
  (if Hit
    (return (Math|Transform|TransformDirection (Transformation|GetActorTransform) (* (Math|Vector|MakeVector 0.0 (Math|Trig|Sin(Degrees) _returnvalue_2) (* (Math|Trig|Cos(Degrees) _returnvalue_2) 1.0)) (Math|Random|RandomFloatinRange 0.0 25.0))))
    (else
      (return (Math|Transform|TransformDirection (Transformation|GetActorTransform) (* (Math|Vector|MakeVector 0.0 (Math|Trig|Sin(Degrees) _returnvalue) (* (Math|Trig|Cos(Degrees) _returnvalue) 1.0)) (Math|Random|RandomFloatinRange 4e+01 8e+01)))))))

(fn HitbyBlaster
  (switch Utilities|FlowControl|Switch|SwitchonWeaponTypes (Variables|Default|GetEquippedWeaponType)
    (:NewEnumerator1
      (Animation|PlayAnimMontage "/Game/AnimStarterPack/Hit.Hit" 1.0 "None"))))

(fn QueueAttack
  (Utilities|Array|Add (Variables|Default|GetActionArray) "NewEnumerator0")
  (bind _asbp_default_game_mode (Utilities|Casting|CastToBP_DefaultGameMode (Game|GetGameMode)))
  (bind _returnvalue (UserInterface|CreateWidget "/Game/UI_Widgets/BP_ActionWidget.BP_ActionWidget_C"))
  (Class|ListView|AddItem (Variables|/Game/UI_Widgets/MainUIWidget.MainUIWidget_C|GetActionQueue_TileView (Variables|/Game/Blueprints/BP_DefaultGameMode.BP_DefaultGameMode_C|GetMainUI _asbp_default_game_mode)) _returnvalue))

(fn RemoveFinishedAction
  (bind _returnvalue (Game|GetGameMode))
  (bind _asbp_default_game_mode (Utilities|Casting|CastToBP_DefaultGameMode _returnvalue))
  (bind _mainui (Variables|/Game/Blueprints/BP_DefaultGameMode.BP_DefaultGameMode_C|GetMainUI _asbp_default_game_mode))
  (bind _actionqueue_tileview (Variables|/Game/UI_Widgets/MainUIWidget.MainUIWidget_C|GetActionQueue_TileView _mainui))
  (Utilities|Array|RemoveIndex (Variables|Default|GetActionArray))
  (Class|ListView|RemoveItem _actionqueue_tileview (Class|ListView|GetItemat _actionqueue_tileview))
  (if (== (Utilities|Array|Length (Variables|Default|GetActionArray)) 0)
    (CallFunction|QueueAttack)))

(fn EndDialogue
  (Variables|Default|SetIsInDialogue false)
  (Variables|Default|SetDisableMovement false)
  (Components|Activation|Deactivate (Variables|Default|GetDialogueCamera))
  (Components|Activation|Activate (Variables|Default|GetCamera) false))

(fn StartDialogue
  (bind _dialoguespringarm (Variables|Default|GetDialogueSpringArm))
  (Variables|Default|SetIsInDialogue true)
  (Variables|Default|SetDisableMovement true)
  (Components|Activation|Deactivate (Variables|Default|GetCamera))
  (Components|Activation|Activate (Variables|Default|GetDialogueCamera) false)
  (bind _returnvalue (Utilities|GetDataTableRow "/Game/CameraAnglesDataTable.CameraAnglesDataTable" "OverShoulderRight")
    (:then
      (Transformation|SetRelativeTransform _dialoguespringarm (.Transform (Utilities|Struct|BreakCameraAngleStruct _returnvalue)) false true)
      (Variables|/Script/Engine.SpringArmComponent|SetTargetArmLength _dialoguespringarm (.ArmLength (Utilities|Struct|BreakCameraAngleStruct _returnvalue))))))
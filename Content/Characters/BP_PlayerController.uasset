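; Player controller Blueprint that lets the player cycle control between party characters with the Tab key.
; Each press increments CurrentPossessionIndex, wraps it against the bounds of the PartyArray held by BP_DefaultGameMode, and has player controller 0 possess that entry.
; Only the lookup value is wrapped, so the stored index keeps growing.
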(event EventBeginPlay)

(event EventTick
  (params (DeltaSeconds :type Float%20%28single-precision%29)))

(event Input|KeyboardEvents|Tab
  (params (Key :type Key%20Structure))
  (bind _returnvalue (Game|GetGameMode))
  (bind _asbp_default_game_mode (Utilities|Casting|CastToBP_DefaultGameMode _returnvalue))
  (bind _partyarray (Variables|/Game/Blueprints/BP_DefaultGameMode.BP_DefaultGameMode_C|GetPartyArray _asbp_default_game_mode))
  ;[1 1 1] Use Tab to cycle through characters
  (:Pressed
    (bind _result (Math|Integer|IncrementInt (Variables|Default|GetCurrentPossessionIndex))
      (:%20%20
        (Pawn|Possess (Game|GetPlayerController 0) (Utilities|Array|Get(acopy) _partyarray (Class|KismetMathLibrary|Wrap _result -1 (- (Utilities|Array|Length _partyarray) 1))))))))

(fn ConstructionScript)
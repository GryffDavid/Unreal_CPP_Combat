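; BP_Door is a sliding double door that opens from an in-world widget button and closes itself after a short delay.
; On BeginPlay it binds the OpenDoor widget's click to a timeline that slides both panels apart, and a timer later reverses it.
; The widget is set visible once closing finishes.
; The construction script passes the trigger sphere and widget to UIToggleTrigger.
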(event Custom|OpenDoor_Event
  ;[1 1 1] Close Doors after a few seconds
  (Utilities|Time|SetTimerbyEvent (delegate Custom|CloseDoor_Event) 5.0)
  ;[1 1 1] Open Doors
  (bind (_direction _door_position) (Timeline|OpenDoors PlayFromStart)
    (:Update
      (Transformation|SetRelativeLocation (Variables|Default|GetLeftDoor) (Math|Vector|MakeVector 0.0 (- 0.0 _door_position) 0.0) false false)
      (Transformation|SetRelativeLocation (Variables|Default|GetRightDoor) (Math|Vector|MakeVector 0.0 _door_position 0.0) false false))
    (:Finished
      (switch Utilities|FlowControl|Switch|SwitchonETimelineDirection _direction
        (:Backward
          (Widget|SetVisibility (UserInterface|GetUserWidgetObject (Variables|Default|GetOpenDoorWidget)) "Visible"))))))

(event Custom|CloseDoor_Event
  ;[1 1 1] Close Doors after a few seconds
  ;[1 1 1] Open Doors
  (bind (_direction _door_position) (Timeline|OpenDoors Reverse)
    (:Update
      (Transformation|SetRelativeLocation (Variables|Default|GetLeftDoor) (Math|Vector|MakeVector 0.0 (- 0.0 _door_position) 0.0) false false)
      (Transformation|SetRelativeLocation (Variables|Default|GetRightDoor) (Math|Vector|MakeVector 0.0 _door_position 0.0) false false))
    (:Finished
      (switch Utilities|FlowControl|Switch|SwitchonETimelineDirection _direction
        (:Backward
          (Widget|SetVisibility (UserInterface|GetUserWidgetObject (Variables|Default|GetOpenDoorWidget)) "Visible"))))))

(event EventBeginPlay
  ;[1 1 1] Get OpenDoorWidget
  (bind _asopen_door_widget (Utilities|Casting|CastToOpenDoorWidget (UserInterface|GetUserWidgetObject (Variables|Default|GetOpenDoorWidget))))
  (EventDispatchers|BindEventtoOpenDoorButtonClicked _asopen_door_widget (delegate Custom|OpenDoor_Event)))

(fn ConstructionScript
  (CallFunction|UIToggleTrigger (Variables|Default|GetUITriggerSphere) (Variables|Default|GetOpenDoorWidget)))
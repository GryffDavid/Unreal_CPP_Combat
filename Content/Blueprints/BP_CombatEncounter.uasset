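; BP_CombatEncounter runs a turn-based combat encounter between the player and the enemy actors attached to it.
; On BeginPlay it registers those enemies; StartCombat rolls a d20 initiative for everyone, sorts enemies highest first and inserts the player, who wins ties.
; DoTurn triggers an enemy's attack or flags the player's turn.
; EndTurn waits briefly, then advances through the combat order, wrapping around.
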(event Custom|StartCombat_Event
  (bind _returnvalue (Game|GetPlayerCharacter 0))
  (bind _asbp_third_person_character (Utilities|Casting|CastToBP_ThirdPersonCharacter _returnvalue))
  ;[1 1 1] StartCombat
  (bind _returnvalue_2 (Class|DiceRoll|RollD20 1))
  (Variables|/Game/Blueprints/BP_ThirdPersonCharacter.BP_ThirdPersonCharacter_C|SetInitiativeRoll _asbp_third_person_character _returnvalue_2)
  (Variables|/Game/Blueprints/BP_ThirdPersonCharacter.BP_ThirdPersonCharacter_C|SetCurrentCombatEncounter _asbp_third_person_character self)
  (for _array_element (Variables|Default|GetEnemies)
    (bind _returnvalue_3 (Class|DiceRoll|RollD20 1))
    (Variables|/Game/Enemies/BP_EnemyBaseClass.BP_EnemyBaseClass_C|SetInitiativeRoll _array_element _returnvalue_3))
  (CallFunction|SortEnemiesbyInitiative) ; After this node is run, CombatOrder contains all \nthe enemies in the encounter sorted by their initiative rolls,\nbut does not contain the player character yet
  (CallFunction|InsertPlayer)
  (Variables|Default|SetCombatStarted true)
  (CallFunction|DoTurnEvent))

(event Custom|DoTurn_Event
  (bind _currentcombatantindex (Variables|Default|GetCurrentCombatantIndex))
  (bind _combatorder (Variables|Default|GetCombatOrder))
  (bind _output (Utilities|Array|Get(acopy) _combatorder _currentcombatantindex))
  ;[1 1 1] DoTurn
  (bind _asbp_enemy_base_class (Utilities|Casting|CastToBP_EnemyBaseClass _output)
    (:then
      (Default|AttackFunction _asbp_enemy_base_class))
    (:CastFailed
      (bind _asbp_third_person_character (Utilities|Casting|CastToBP_ThirdPersonCharacter _output))
      (Variables|/Game/Blueprints/BP_ThirdPersonCharacter.BP_ThirdPersonCharacter_C|SetIsMyTurn _asbp_third_person_character true))))

(event Custom|EndTurn_Event
  ;[1 1 1] EndTurn
  (Utilities|FlowControl|Delay 1.6)
  (bind _result (Math|Integer|IncrementInt (Variables|Default|GetCurrentCombatantIndex))
    (:%20%20
      (if (>= _result (Utilities|Array|Length (Variables|Default|GetCombatOrder)))
        (Variables|Default|SetCurrentCombatantIndex 0))
      (CallFunction|DoTurnEvent))))

(event EventBeginPlay
  (for _array_element (Actor|GetAttachedActors true)
    (bind _asbp_enemy_base_class (Utilities|Casting|CastToBP_EnemyBaseClass _array_element))
    (Utilities|Array|AddUnique (Variables|Default|GetEnemies) _asbp_enemy_base_class)
    (Variables|/Game/Enemies/BP_EnemyBaseClass.BP_EnemyBaseClass_C|SetEncounterContainer _asbp_enemy_base_class self)))

(fn ConstructionScript)

(fn SortEnemiesbyInitiative
  (LocalVariables|SetTempOrder (Variables|Default|GetEnemies))
  (while (> (Utilities|Array|Length (LocalVariables|GetTempOrder)) 0)
    (bind _enemywithhighestinitiative (CallFunction|GetEnemywithHighestInitiative (LocalVariables|GetTempOrder)))
    (Utilities|Array|AddUnique (Variables|Default|GetCombatOrder) _enemywithhighestinitiative)
    (Utilities|Array|RemoveItem (LocalVariables|GetTempOrder) _enemywithhighestinitiative)))

(fn GetEnemywithHighestInitiative
  (params (Array :type Array%20of%20BP%20Enemy%20Base%20Class%20Object%20References))
  (for (_array_element _array_index) Array
    (if (> (Variables|/Game/Enemies/BP_EnemyBaseClass.BP_EnemyBaseClass_C|GetInitiativeRoll _array_element) (LocalVariables|GetHighestInitiative))
      (LocalVariables|SetHighestInitiative (Variables|/Game/Enemies/BP_EnemyBaseClass.BP_EnemyBaseClass_C|GetInitiativeRoll _array_element))
      (LocalVariables|SetMaxInitiativeIndex _array_index)))
  (return (Utilities|Array|Get(acopy) Array (LocalVariables|GetMaxInitiativeIndex))))

(fn InsertPlayer
  (bind _returnvalue (Game|GetPlayerCharacter 0))
  (bind _combatorder (Variables|Default|GetCombatOrder))
  (bind _asbp_third_person_character (Utilities|Casting|CastToBP_ThirdPersonCharacter _returnvalue))
  (bind (_array_element _array_index) (Utilities|Array|ForEachLoopwithBreak (Variables|Default|GetCombatOrder) :!label _label)
    (:LoopBody
      (if (>= (Variables|/Game/Blueprints/BP_ThirdPersonCharacter.BP_ThirdPersonCharacter_C|GetInitiativeRoll (.AsBP%20Third%20Person%20Character (Utilities|Casting|CastToBP_ThirdPersonCharacter (Game|GetPlayerCharacter 0)))) (Variables|/Game/Enemies/BP_EnemyBaseClass.BP_EnemyBaseClass_C|GetInitiativeRoll (.AsBP%20Enemy%20Base%20Class (Utilities|Casting|CastToBP_EnemyBaseClass _array_element))))
        (LocalVariables|SetInsertPlayerIndex _array_index)
        (goto _label Break)))
    (:Completed
      (if (== (LocalVariables|GetInsertPlayerIndex) -1)
        (Utilities|Array|AddUnique _combatorder _asbp_third_person_character)
        (else
          (Utilities|Array|Insert _combatorder _asbp_third_person_character (LocalVariables|GetInsertPlayerIndex)))))))
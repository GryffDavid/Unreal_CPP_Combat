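; BP_Enemy is an enemy character that can be clicked as a target, paused and killed by blaster bolts.
; Clicking its mesh passes it to the third-person player character's target-click event.
; A bolt hit starts a reaction animation, mesh physics and an impulse at the feet marker, then calls OnDeathEvent; a death handler clears targeting and ragdolls the body.
; The pause event toggles skeleton updates and character movement.
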(event OnClicked(Mesh)
  (params (TouchedComponent :type Primitive%20Component%20Object%20Reference) (ButtonPressed :type Key%20Structure :default "None"))
  (bind _asbp_third_person_character (Utilities|Casting|CastToBP_ThirdPersonCharacter (Game|GetPlayerCharacter 0)))
  (Default|TargetClickedEvent _asbp_third_person_character self))

(event Custom|OnDeath_Event
  (bind _mesh (Variables|Character|GetMesh))
  (Rendering|SetVisibility (Variables|Default|GetAttackWidget) false false)
  (Variables|Default|SetIsTargeted false)
  ;[1 1 1] Go Ragdolll on Death
  (Collision|SetCollisionEnabled (Variables|Default|GetCapsuleComponent) "NoCollision")
  (Physics|SetSimulatePhysics _mesh true)
  (Collision|SetCollisionEnabled _mesh "PhysicsOnly")
  (Physics|AddForce _mesh "500.000000,-500000.000000,500000.000000" (Class|SkinnedMeshComponent|GetBoneName _mesh 3) false))

(event Custom|ToggleEnemyPause_Event
  (bind _output_get (Variables|Default|SetActivePause (not (Variables|Default|GetActivePause))))
  (Variables|/Script/Engine.SkeletalMeshComponent|SetbNoSkeletonUpdate (Variables|Character|GetMesh) _output_get)
  (Components|Activation|ToggleActive (Variables|Character|GetCharacterMovement)))

(event EventBeginPlay)

(event Collision|EventActorBeginOverlap
  (params (OtherActor :type Actor%20Object%20Reference)))

(event EventTick
  (params (DeltaSeconds :type Float%20%28single-precision%29)))

(event Collision|EventHit
  (params (MyComp :type Primitive%20Component%20Object%20Reference) (Other :type Actor%20Object%20Reference) (OtherComp :type Primitive%20Component%20Object%20Reference) (bSelfMoved :type Boolean) (HitLocation :type Vector :default "0, 0, 0") (HitNormal :type Vector :default "0, 0, 0") (NormalImpulse :type Vector :default "0, 0, 0") (Hit :type Hit%20Result%20Structure%20%28by%20ref%29))
  (bind _mesh (Variables|Character|GetMesh))
  (Utilities|Casting|CastToBP_BlasterBoltProjectile Other)
  (Components|Animation|PlayAnimation (Variables|Character|GetMesh) "/Game/AnimStarterPack/Hit_React_3.Hit_React_3" false)
  (Physics|SetSimulatePhysics _mesh true)
  (Physics|AddImpulseatLocation _mesh (* "-12.000000,0.000000,12.000000" 1e+03) (Transformation|GetWorldLocation (Variables|Default|GetFeetMarker)) "None")
  (CallFunction|OnDeathEvent))

(fn ConstructionScript)
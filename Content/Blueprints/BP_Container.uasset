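; BP_Container is a container actor with an attached widget for an open-container UI.
; On BeginPlay it runs the parent logic, casts the widget component's user widget to OpenContainerWidget and passes itself in as that widget's Container.
; OpenContainer and CloseContainer are empty function stubs, so no opening or closing behavior is implemented here.
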(event EventBeginPlay
  (|CallParentFunction)
  (bind _asopen_container_widget (Utilities|Casting|CastToOpenContainerWidget (UserInterface|GetUserWidgetObject (Variables|Default|GetWidget))))
  (Variables|/Game/UI_Widgets/OpenContainerWidget.OpenContainerWidget_C|SetContainer _asopen_container_widget self))

(event Collision|EventActorBeginOverlap
  (params (OtherActor :type Actor%20Object%20Reference))
  (|CallParentFunction OtherActor) ; This node is disabled and will not be called.\nDrag off pins to build functionality.
)

(event EventTick
  (params (DeltaSeconds :type Float%20%28single-precision%29))
  (|CallParentFunction DeltaSeconds) ; This node is disabled and will not be called.\nDrag off pins to build functionality.
)

(fn ConstructionScript
  (|CallParentFunction))

(fn OpenContainer)

(fn CloseContainer)
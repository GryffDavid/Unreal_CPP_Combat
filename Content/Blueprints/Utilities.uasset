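; Utility functions that look up an item's row in ItemDataTable from either an item class or an item object.
; The row name is the class display name with its last two characters chopped, so rows are keyed by class name without the `_C` suffix.
; The object variant first casts the object's class to ItemBaseClass.
; Both wire a return only for the Row Found case.
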(fn GetItemDatabyClass
  (params (ItemClass :type Item%20Base%20Class%20Class%20Reference))
  (bind _returnvalue (Utilities|GetDataTableRow "/Game/ItemDataTable.ItemDataTable" (Utilities|String|StringToName (Utilities|String|LeftChop (Utilities|GetClassDisplayName ItemClass) 2)))
    (:then
      (return _returnvalue))))

(fn GetItemDatabyObject
  (params (ItemObject :type Object%20Object%20Reference))
  (bind _returnvalue (Utilities|GetDataTableRow "/Game/ItemDataTable.ItemDataTable" (Utilities|String|StringToName (Utilities|String|LeftChop (Utilities|GetClassDisplayName (.AsItem%20Base%20Class (Utilities|Casting|CastToItemBaseClassClass (Utilities|GetClass ItemObject)))) 2)))
    (:then
      (return _returnvalue))))
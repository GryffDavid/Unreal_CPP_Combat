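; Default game mode Blueprint that owns the active-pause state and sets up the main UI.
; BeginPlay creates the MainUIWidget, stores it as MainUI and adds it to the viewport.
; ToggleActivePause_Event flips IsActivePaused, then gathers every BlasterBoltProjectile with GetAllActorsOfClass and passes the new state to each one's ToggleActivePause.
; Only projectiles are notified here, with no global game pause.
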(event Custom|ToggleActivePause_Event
  (bind _output_get (Variables|Default|SetIsActivePaused (not (Variables|Default|GetIsActivePaused))))
  (bind _outactors (Actor|GetAllActorsOfClass "/Script/Unreal_CPP_Combat.BlasterBoltProjectile"))
  (for _array_element _outactors
    (bind _asblaster_bolt_projectile (Utilities|Casting|CastToBlasterBoltProjectile _array_element))
    (Class|BlasterBoltProjectile|ToggleActivePause _asblaster_bolt_projectile _output_get)))

(event EventBeginPlay
  (bind _returnvalue (UserInterface|CreateWidget "/Game/UI_Widgets/MainUIWidget.MainUIWidget_C"))
  (bind _output_get (Variables|Default|SetMainUI _returnvalue))
  (UserInterface|Viewport|AddtoViewport _output_get 0))

(event EventTick
  (params (DeltaSeconds :type Float%20%28single-precision%29)))

(fn ConstructionScript)
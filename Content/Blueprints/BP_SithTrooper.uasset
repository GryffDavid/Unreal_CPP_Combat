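; BP_SithTrooper is a clickable enemy with HP, an attack widget and an active-pause mode.
; Clicking its mesh reports it to the player character as a target; while targeted and unpaused, it takes damage from blaster bolts flagged to hit.
; AdjustHP triggers death at zero HP, where the death handler hides the widget and launches the body as a ragdoll.
; Pause toggling freezes skeleton updates and toggles character movement.
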(event OnClicked(Mesh)
  (params (TouchedComponent :type Primitive%20Component%20Object%20Reference) (ButtonPressed :type Key%20Structure :default "None"))
  (bind _asbp_third_person_character (Utilities|Casting|CastToBP_ThirdPersonCharacter (Game|GetPlayerCharacter 0)))
  (Default|TargetClickedEvent _asbp_third_person_character self))

(event Custom|OnDeath_Event
  (bind _mesh (Variables|Character|GetMesh))
  ;[1 1 1] Make widget invisible on death
  (Rendering|SetVisibility (Variables|Default|GetAttackWidget) false false)
  (Variables|Default|SetIsTargeted false)
  ;[1 1 1] Go Ragdolll on Death
  (Collision|SetCollisionEnabled (Variables|Default|GetCapsuleComponent) "NoCollision")
  (Physics|SetSimulatePhysics _mesh true)
  (Collision|SetCollisionEnabled _mesh "PhysicsOnly")
  (Physics|AddForce _mesh "500.000000,-500000.000000,500000.000000" (Class|SkinnedMeshComponent|GetBoneName _mesh 3) false))

(event Custom|ToggleEnemyPause_Event
  (bind _output_get (Variables|Default|SetActivePause (not (Variables|Default|GetActivePause))))
  (Variables|/Script/Engine.SkeletalMeshComponent|SetbNoSkeletonUpdate (Variables|Character|GetMesh) _output_get)
  (Components|Activation|ToggleActive (Variables|Character|GetCharacterMovement)))

(event EventBeginPlay
  (bind _asattack_widget (Utilities|Casting|CastToAttackWidget (UserInterface|GetWidget (Variables|Default|GetAttackWidget))))
  (Variables|/Game/UI_Widgets/AttackWidget.AttackWidget_C|SetEnemyAttachedTo _asattack_widget self))

(event Collision|EventActorBeginOverlap
  (params (OtherActor :type Actor%20Object%20Reference))
  ;[1 1 1] Overlapped with Blaster bolt. Ignore if is not current target or shot is meant to miss
  (if (not (Variables|Default|GetActivePause))
    (bind _asbp_blaster_bolt_projectile (Utilities|Casting|CastToBP_BlasterBoltProjectile OtherActor))
    (if (and (Variables|/Game/Blueprints/BP_BlasterBoltProjectile.BP_BlasterBoltProjectile_C|GetCanHit _asbp_blaster_bolt_projectile) (Variables|Default|GetIsTargeted))
      (Actor|DestroyActor _asbp_blaster_bolt_projectile)
      (Components|Animation|PlayAnimation (Variables|Character|GetMesh) "/Game/AnimStarterPack/Hit_React_1.Hit_React_1" false)
      (CallFunction|AdjustHP 6))))

(fn ConstructionScript)

(fn AdjustHP
  (params (Change :type Integer))
  (Variables|Default|SetCurrentHP (- (Variables|Default|GetCurrentHP) Change))
  (bind _output_get (Variables|Default|SetHPPercent (/ (Math|Conversions|ToFloat(Integer) (Variables|Default|GetCurrentHP)) (Math|Conversions|ToFloat(Integer) (Variables|Default|GetMaxHP)))))
  (if (<= _output_get 0.0)
    (CallFunction|OnDeathEvent))
  (return))
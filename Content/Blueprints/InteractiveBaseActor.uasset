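; InteractiveBaseActor is an interactive actor, apparently a base class, that shows its Widget when the player is nearby with an unobstructed view.
; Each Tick it compares the distance from the player character's HeadMarker to its root against the Sphere's unscaled radius, without using overlap events.
; In range, a debug-drawn Visibility trace runs from head to root, ignoring the player; any hit hides the Widget, as does being out of range.
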(event EventBeginPlay)

(event Collision|EventActorBeginOverlap
  (params (OtherActor :type Actor%20Object%20Reference)))

(event EventTick
  (params (DeltaSeconds :type Float%20%28single-precision%29))
  (bind _returnvalue (Game|GetPlayerCharacter 0))
  (bind _rootcomponent (Variables|Transformation|GetRootComponent))
  (bind _widget (Variables|Default|GetWidget))
  (bind _returnvalue_2 (Transformation|GetWorldLocation _rootcomponent))
  (bind _asbp_third_person_character (Utilities|Casting|CastToBP_ThirdPersonCharacter _returnvalue))
  (bind _headmarker (Variables|/Game/Blueprints/BP_ThirdPersonCharacter.BP_ThirdPersonCharacter_C|GetHeadMarker _asbp_third_person_character))
  (bind _returnvalue_3 (Transformation|GetWorldLocation _headmarker))
  (if (> (Math|Vector|Distance(Vector) _returnvalue_3 _returnvalue_2) (Class|SphereComponent|GetUnscaledSphereRadius (Variables|Default|GetSphere)))
    (Rendering|SetVisibility _widget false false :!label _label)
    (else
      (bind _returnvalue_4 (Collision|LineTraceByChannel _returnvalue_3 _returnvalue_2 "TraceTypeQuery1" false (Utilities|Array|MakeArray _returnvalue) "ForOneFrame"))
      (if _returnvalue_4
        (goto _label)
        (else
          (Rendering|SetVisibility _widget true false))))))

(fn ConstructionScript)
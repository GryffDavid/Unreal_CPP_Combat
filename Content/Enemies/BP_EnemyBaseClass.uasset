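; Base enemy class for encounter-based combat with click targeting and placeholder attack and hit-reaction hooks.
; An unobstructed trace from the player's head marks the encounter seen and pauses; AI perception of the player locks movement, pauses and starts combat through EncounterContainer.
; Blaster bolts damage only the targeted enemy when flagged to hit, and death removes it from the encounter.
; AddRandomMiss returns random offsets, tight for hits and wider for misses.
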(event OnTargetPerceptionUpdated(AIPerception)
  (params (Actor :type Actor%20Object%20Reference) (Stimulus :type AI%20Stimulus%20Structure))
  ;[1 1 1] Enemy spotted the player?
  (bind _asbp_character_base_class (Utilities|Casting|CastToBP_CharacterBaseClass Actor))
  (if (and (.bSuccessfullySensed (Utilities|Struct|BreakAIStimulus Stimulus)) (not (Variables|Default|GetInCombat)))
    ;[1 1 1] Disable player movement, set everyone to "IN COMBAT" and start the combat sequence
    (Variables|/Game/Characters/BP_CharacterBaseClass.BP_CharacterBaseClass_C|SetInCombat _asbp_character_base_class true)
    (Variables|/Script/Unreal_CPP_Combat.CharacterBaseClass|SetDisableMovement _asbp_character_base_class true)
    (Game|SetGamePaused true)
    (for _array_element (Variables|/Game/Blueprints/BP_CombatEncounter.BP_CombatEncounter_C|GetEnemies (Variables|Default|GetEncounterContainer))
      (Variables|BP_EnemyBaseClass_C|SetInCombat _array_element true))
    (Default|StartCombatEvent (Variables|Default|GetEncounterContainer))))

(event OnClicked(Mesh)
  (params (TouchedComponent :type Primitive%20Component%20Object%20Reference) (ButtonPressed :type Key%20Structure))
  ;[1 1 1] Enemy was clicked
  (bind _asbp_character_base_class (Utilities|Casting|CastToBP_CharacterBaseClass (Game|GetPlayerCharacter 0)))
  (Variables|/Game/Characters/BP_CharacterBaseClass.BP_CharacterBaseClass_C|SetTargetedEnemy _asbp_character_base_class self))

(event OnBeginCursorOver(Mesh)
  (params (TouchedComponent :type Primitive%20Component%20Object%20Reference)))

(event Custom|StartCombat)

(event EventBeginPlay
  ;[1 1 1] Setup the attack widget
  (bind _asbp_attack_widget (Utilities|Casting|CastToBP_AttackWidget (UserInterface|GetWidget (Variables|Default|GetWidgetComponent))))
  (Variables|/Game/UI_Widgets/BP_AttackWidget.BP_AttackWidget_C|SetEnemyAttachedTo _asbp_attack_widget self))

(event Collision|EventActorBeginOverlap
  (params (OtherActor :type Actor%20Object%20Reference))
  ;[1 1 1] Overlapped with Blaster bolt. Ignore if is not current target or shot is meant to miss
  (bind _asbp_blaster_bolt_projectile (Utilities|Casting|CastToBP_BlasterBoltProjectile OtherActor))
  (if (and (Variables|/Script/Unreal_CPP_Combat.BlasterBoltProjectile|GetCanHit _asbp_blaster_bolt_projectile) (Variables|Default|GetIsTargeted))
    (bind _returnvalue (Class|EnemyBaseClass|DecreaseHP (Variables|/Game/Blueprints/BP_BlasterBoltProjectile.BP_BlasterBoltProjectile_C|GetDamageToDo _asbp_blaster_bolt_projectile)))
    (if _returnvalue
      (CallFunction|DeathBehaviour)
      (else
        (CallFunction|HitbyBlaster)))
    (Effects|SpawnEmitteratLocation "/Game/P_Sparks.P_Sparks" (Transformation|GetActorLocation _asbp_blaster_bolt_projectile))
    (Actor|DestroyActor _asbp_blaster_bolt_projectile)))

(event EventTick
  (params (DeltaSeconds :type Float%20%28single-precision%29))
  ;[1 1 1] Has the player spotted this enemy yet?
  (bind _returnvalue (Collision|LineTraceByChannel (Transformation|GetWorldLocation (Variables|/Game/Characters/BP_CharacterBaseClass.BP_CharacterBaseClass_C|GetHeadMarker (.AsBP%20Character%20Base%20Class (Utilities|Casting|CastToBP_CharacterBaseClass (Game|GetPlayerCharacter 0))))) (Transformation|GetWorldLocation (Variables|Transformation|GetRootComponent)) "TraceTypeQuery1" false 0 "None"))
  (if (not _returnvalue)
    (if (not (Variables|Default|GetWasSeen))
      (Utilities|FlowControl|DoOnce false
        (:Completed
          (for _array_element (Variables|/Game/Blueprints/BP_CombatEncounter.BP_CombatEncounter_C|GetEnemies (Variables|Default|GetEncounterContainer))
            (Variables|BP_EnemyBaseClass_C|SetWasSeen _array_element true))
          (Game|SetGamePaused true))))))

(fn ConstructionScript)

(fn HitbyBlaster)

(fn DeathBehaviour
  (Utilities|Array|RemoveItem (Variables|/Game/Blueprints/BP_CombatEncounter.BP_CombatEncounter_C|GetCombatOrder (Variables|Default|GetEncounterContainer)) self)
  (Utilities|Array|RemoveItem (Variables|/Game/Blueprints/BP_CombatEncounter.BP_CombatEncounter_C|GetEnemies (Variables|Default|GetEncounterContainer)) self))

(fn AddRandomMiss
  (params (Hit :type Boolean))
  (bind _returnvalue (Math|Random|RandomFloatinRange -1.1e+02 1.1e+02))
  (bind _returnvalue_2 (Math|Random|RandomFloatinRange 0.0 3.6e+02))
  (if Hit
    (return (Math|Transform|TransformDirection (Transformation|GetActorTransform) (* (Math|Vector|MakeVector 0.0 (Math|Trig|Sin(Degrees) _returnvalue_2) (* (Math|Trig|Cos(Degrees) _returnvalue_2) 1.0)) (Math|Random|RandomFloatinRange 0.0 25.0))))
    (else
      (return (Math|Transform|TransformDirection (Transformation|GetActorTransform) (* (Math|Vector|MakeVector 0.0 (Math|Trig|Sin(Degrees) _returnvalue) (* (Math|Trig|Cos(Degrees) _returnvalue) 1.0)) (Math|Random|RandomFloatinRange 4e+01 8e+01)))))))

(fn AttackFunction)
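; Sith heavy trooper enemy that reacts to blaster hits with a hit montage and dies into a physics ragdoll.
; DeathBehaviour fires an event that switches off capsule collision, sets the mesh to physics-only and runs the PlayRandomDeathAnimation macro.
; The macro either plays one of three death animations, drops the gun as a physics object and waits a random delay, or skips straight to ragdoll without detaching the gun.
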(event Custom|DeathFunctionality_Event
  (bind _mesh (Variables|Character|GetMesh))
  (Collision|SetCollisionEnabled (Variables|Default|GetCapsuleComponent) "NoCollision")
  (Collision|SetCollisionEnabled _mesh "PhysicsOnly")
  (Utilities|PlayRandomDeathAnimation
    (:OutputPin
      (Physics|SetSimulatePhysics _mesh true))))

(event EventBeginPlay)

(event Collision|EventActorBeginOverlap
  (params (OtherActor :type Actor%20Object%20Reference))
  (|CallParentFunction OtherActor) ; This node is disabled and will not be called.\nDrag off pins to build functionality.
)

(event EventTick
  (params (DeltaSeconds :type Float%20%28single-precision%29)))

(fn ConstructionScript
  (|CallParentFunction))

(fn HitbyBlaster
  (Animation|PlayAnimMontage "/Game/AnimStarterPack/Hit.Hit" 1.0 "None"))

(fn DeathBehaviour
  (CallFunction|DeathFunctionalityEvent))
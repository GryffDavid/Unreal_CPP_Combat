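; Sith trooper enemy that periodically shoots blaster bolts at the player using tabletop-style dice rolls.
; From BeginPlay, a randomly delayed loop rolls a D20 against the player's Dexterity, setting the bolt's hit flag, D6 damage and aim offset from the chest marker.
; Blaster hits play a reaction animation.
; Death disables capsule collision, then ragdolls the mesh immediately or shortly into a random death animation.
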(event Custom|DeathFunctionality_Event
  (bind _mesh (Variables|Character|GetMesh))
  (Collision|SetCollisionEnabled (Variables|Default|GetCapsuleComponent) "NoCollision")
  (Collision|SetCollisionEnabled _mesh "PhysicsOnly")
  (Utilities|PlayRandomDeathAnimation
    (:OutputPin
      (Physics|SetSimulatePhysics _mesh true))))

(event EventBeginPlay
  (|CallParentFunction)
  (Variables|Default|SetTargetedEnemy (Game|GetPlayerCharacter 0))
  (while (< (Variables|Default|GetNewVar_0) 9000)
    (Math|Integer|IncrementInt (Variables|Default|GetNewVar_0)
      (:%20%20
        (Utilities|FlowControl|Delay (Math|Random|RandomFloatinRange 3.0 8.0))
        (CallFunction|AttackFunction)))))

(event Collision|EventActorBeginOverlap
  (params (OtherActor :type Actor%20Object%20Reference))
  (|CallParentFunction OtherActor) ; This node is disabled and will not be called.\nDrag off pins to build functionality.
)

(event EventTick
  (params (DeltaSeconds :type Float%20%28single-precision%29))
  (|CallParentFunction DeltaSeconds) ; This node is disabled and will not be called.\nDrag off pins to build functionality.
)

(fn ConstructionScript
  (|CallParentFunction))

(fn HitbyBlaster
  (Components|Animation|PlayAnimation (Variables|Character|GetMesh) "/Game/AnimStarterPack/Hit_React_1.Hit_React_1" false))

(fn DeathBehaviour
  (CallFunction|DeathFunctionalityEvent))

(fn AttackFunction
  (bind _targetedenemy (Variables|Default|GetTargetedEnemy))
  (bind _gunbarrel (Variables|Default|GetGunBarrel))
  (bind _returnvalue (Transformation|GetWorldLocation _gunbarrel))
  (bind _asbp_third_person_character (Utilities|Casting|CastToBP_ThirdPersonCharacter _targetedenemy))
  (bind _returnvalue_2 (Class|DiceRoll|RollD20vDC (Variables|/Script/Unreal_CPP_Combat.ThirdPersonCharacter|GetDexterity _asbp_third_person_character) 0 1))
  (bind _returnvalue_3 (CallFunction|AddRandomMiss _returnvalue_2))
  (if _returnvalue_2
    (bind _returnvalue_4 (Class|DiceRoll|RollD6 1)))
  (Game|SpawnActorfromClass "/Game/Blueprints/BP_EnemyBlasterBoltProjectile.BP_EnemyBlasterBoltProjectile_C" (Math|Transform|MakeTransform _returnvalue (Math|Conversions|RotationFromXVector (Math|Vector|GetUnitDirection(Vector) _returnvalue (+ (Transformation|GetWorldLocation (Variables|/Game/Blueprints/BP_ThirdPersonCharacter.BP_ThirdPersonCharacter_C|GetChestMarker _asbp_third_person_character)) _returnvalue_3)))) "Undefined" 0 _returnvalue_2 _returnvalue_4 0))